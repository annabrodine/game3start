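; Game Instance that saves, loads and deletes player progress and per-level data through two SaveGame classes.
; SaveGame writes stamina, transform and sprint/shoot flags to SG_CodingII; LoadGame restores only stamina and transform, copying flags into the save object instead.
; Init prepares SG_LevelSave from the level-named slot, and LoadLevel, called by LoadGame, applies its collected objects.
; SaveLevel writes that data to an empty slot name, unlike the level-named reads and deletes.
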(event Custom|SaveGame
  (Development|PrintString "Starting Save Game")
  (bind _returnvalue (SaveGame|DoesSaveGameExist (Variables|Default|GetSlot%20Name)))
  (if _returnvalue ; true if we've saved before
    (bind _returnvalue_2 (SaveGame|LoadGamefromSlot (Variables|Default|GetSlot%20Name)))
    (Variables|Default|SetSave%20Subclass _returnvalue_2)
    (else
      (bind _returnvalue_3 (SaveGame|CreateSaveGameObject "/Game/ThirdPerson/Blueprints/SG_CodingII.SG_CodingII_C"))
      (Variables|Default|SetSave%20Subclass _returnvalue_3)))
  (bind _assg_coding_ii (Utilities|Casting|CastToSG_CodingII (Variables|Default|GetSave%20Subclass)))
  (bind _asbp_third_person_character (Utilities|Casting|CastToBP_ThirdPersonCharacter (Game|GetPlayerCharacter 0))
    (:then
      (Variables|/Game/ThirdPerson/Blueprints/SG_CodingII.SG_CodingII_C|SetPlayerStamina _assg_coding_ii (Variables|/Game/ThirdPerson/Blueprints/BP_ThirdPersonCharacter.BP_ThirdPersonCharacter_C|GetStamina _asbp_third_person_character))
      (Variables|/Game/ThirdPerson/Blueprints/SG_CodingII.SG_CodingII_C|SetPlayerTransform _assg_coding_ii (Transformation|GetWorldTransform (Variables|/Script/Engine.Character|GetCapsuleComponent _asbp_third_person_character)))
      (Variables|/Game/ThirdPerson/Blueprints/SG_CodingII.SG_CodingII_C|SetPlayerCanSprint _assg_coding_ii (Variables|/Game/ThirdPerson/Blueprints/BP_ThirdPersonCharacter.BP_ThirdPersonCharacter_C|GetCanSprint _asbp_third_person_character))
      (Variables|/Game/ThirdPerson/Blueprints/SG_CodingII.SG_CodingII_C|SetPlayerCanShoot _assg_coding_ii (Variables|/Game/ThirdPerson/Blueprints/BP_ThirdPersonCharacter.BP_ThirdPersonCharacter_C|GetCanShoot _asbp_third_person_character))
      (SaveGame|SaveGametoSlot _assg_coding_ii (Variables|Default|GetSlot%20Name))
      (Development|PrintString "game successfully saved" true true "(R=0.140382,G=1.000000,B=0.000000,A=1.000000)"))
    (:CastFailed
      (Development|PrintString "Failed"))))

(event Custom|LoadGame
  (Development|PrintString "Starting Load Game")
  (CallFunction|LoadLevel)
  (bind _returnvalue (SaveGame|DoesSaveGameExist (Variables|Default|GetSlot%20Name)))
  (if _returnvalue
    (bind _returnvalue_2 (SaveGame|LoadGamefromSlot (Variables|Default|GetSlot%20Name)))
    (Variables|Default|SetSave%20Subclass _returnvalue_2)
    (bind _assg_coding_ii (Utilities|Casting|CastToSG_CodingII (Variables|Default|GetSave%20Subclass)))
    (bind _asbp_third_person_character (Utilities|Casting|CastToBP_ThirdPersonCharacter (Game|GetPlayerCharacter 0)))
    (Variables|/Game/ThirdPerson/Blueprints/BP_ThirdPersonCharacter.BP_ThirdPersonCharacter_C|SetStamina _asbp_third_person_character (Variables|/Game/ThirdPerson/Blueprints/SG_CodingII.SG_CodingII_C|GetPlayerStamina _assg_coding_ii))
    (Transformation|SetWorldTransform (Variables|/Script/Engine.Character|GetCapsuleComponent _asbp_third_person_character) (Variables|/Game/ThirdPerson/Blueprints/SG_CodingII.SG_CodingII_C|GetPlayerTransform _assg_coding_ii) false false)
    (Variables|/Game/ThirdPerson/Blueprints/SG_CodingII.SG_CodingII_C|SetPlayerCanSprint _assg_coding_ii (Variables|/Game/ThirdPerson/Blueprints/BP_ThirdPersonCharacter.BP_ThirdPersonCharacter_C|GetCanSprint _asbp_third_person_character))
    (Variables|/Game/ThirdPerson/Blueprints/SG_CodingII.SG_CodingII_C|SetPlayerCanShoot _assg_coding_ii (Variables|/Game/ThirdPerson/Blueprints/BP_ThirdPersonCharacter.BP_ThirdPersonCharacter_C|GetCanShoot _asbp_third_person_character))
    (else
      (Development|PrintString "No data"))))

(event Custom|SaveLevel
  (Development|PrintString "saving level from game instance")
  (Game|GetCurrentLevelName true)
  (SaveGame|SaveGametoSlot (Variables|Default|GetLevelData)))

(event Custom|LoadLevel
  (Development|PrintString "loading level from game instance")
  (bind _returnvalue (Game|GetCurrentLevelName true))
  (SaveGame|DoesSaveGameExist _returnvalue)
  (if true
    (Default|LoadCollectedObjects (Variables|Default|GetLevelData))))

(event Custom|Delete%20Save%20Data
  (SaveGame|DeleteGameinSlot (Variables|Default|GetSlot%20Name))
  (bind _returnvalue (Game|GetCurrentLevelName true))
  (SaveGame|DeleteGameinSlot _returnvalue)
  (if true
    (Development|PrintString "successfuly deleted saves")
    (else
      (Development|PrintString "could not delete player save"))))

(event EventInit
  (bind _returnvalue (Game|GetCurrentLevelName true))
  (SaveGame|DoesSaveGameExist _returnvalue)
  (if true
    (bind _returnvalue_2 (SaveGame|LoadGamefromSlot _returnvalue))
    (bind _assg_level_save (Utilities|Casting|CastToSG_LevelSave _returnvalue_2))
    (Variables|Default|SetLevelData _assg_level_save)
    (else
      (bind _returnvalue_3 (SaveGame|CreateSaveGameObject "/Game/Blueprints/SG_LevelSave.SG_LevelSave_C"))
      (Variables|Default|SetLevelData _returnvalue_3))))
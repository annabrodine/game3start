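; Game mode that manages per-level saves through an SG_LevelSave2 object, using the level name as slot name.
; BeginPlay creates a save object or loads one, though loading passes an empty slot name and a failed cast deletes the level's slot.
; A successful load restores collected coins, but applies the saved player transform only when its location is zero.
; Checkpoint stores the player transform and FinishLevel clears it, both then saving.
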(event Custom|SaveGame
  (bind _returnvalue (Game|GetCurrentLevelName true))
  (bind _returnvalue_2 (SaveGame|SaveGametoSlot (Variables|Default|GetLevel%20Save) _returnvalue))
  (if _returnvalue_2
    (Development|PrintString "saved level")
    (else
      (Development|PrintString "could not save level"))))

(event EventBeginPlay
  (Development|PrintString "loaded into the gm ")
  (bind _returnvalue (Game|GetCurrentLevelName true))
  (bind _returnvalue_2 (SaveGame|DoesSaveGameExist _returnvalue))
  (if _returnvalue_2
    (bind _returnvalue_3 (SaveGame|LoadGamefromSlot))
    (bind _assg_level_save_2 (Utilities|Casting|CastToSG_LevelSave2 _returnvalue_3)
      (:then
        (bind _output_get (Variables|Default|SetLevel%20Save _assg_level_save_2))
        (Default|LoadCollectedCoins _output_get)
        (if (Class|KismetMathLibrary|EqualExactlyVectorVector (.location (Variables|/Game/Blueprints/newsaves/SG_LevelSave2.SG_LevelSave2_C|GetPlayerTransform (Variables|Default|GetLevel%20Save))) "0, 0, 0")
          (Transformation|SetWorldTransform (Variables|/Script/Engine.Character|GetCapsuleComponent (Game|GetPlayerCharacter 0)) (Variables|/Game/Blueprints/newsaves/SG_LevelSave2.SG_LevelSave2_C|GetPlayerTransform (Variables|Default|GetLevel%20Save)) false false)))
      (:CastFailed
        (SaveGame|DeleteGameinSlot _returnvalue)))
    (else
      (bind _returnvalue_4 (SaveGame|CreateSaveGameObject "/Game/Blueprints/newsaves/SG_LevelSave2.SG_LevelSave2_C"))
      (Variables|Default|SetLevel%20Save _returnvalue_4))))

(event EventTick
  (params (DeltaSeconds :type Float%20%28single-precision%29)))

(fn ConstructionScript)

(fn Checkpoint
  (params (Player%20Transform :type Transform))
  (Variables|/Game/Blueprints/newsaves/SG_LevelSave2.SG_LevelSave2_C|SetPlayerTransform (Variables|Default|GetLevel%20Save) Player%20Transform)
  (CallFunction|SaveGame))

(fn FinishLevel
  (Variables|/Game/Blueprints/newsaves/SG_LevelSave2.SG_LevelSave2_C|SetPlayerTransform (Variables|Default|GetLevel%20Save) "")
  (CallFunction|SaveGame))